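; Example Blueprint that uses subjects, traits and mechanics to move entities along navmesh paths to random destinations.
; BeginPlay spawns subjects with navmesh-projected random positions and targets.
; Tick mechanics swap the desired-path trait for found path points, set velocity toward the next point, integrate position and debug-draw the results.
; Failed searches retry every tick; reached points are dropped until subjects stop, without choosing new destinations.
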(event `self.ReceiveBeginPlay`
  (bind _projectedlocation (`NavigationSystemV1.K2_ProjectPointToNavigation` (* (* (`KismetMathLibrary.RandomUnitVector`) (`self.RandomSpawnWidth`)) (1.0 1.0 0.0)) null null (1000.0 1000.0 1000.0)))
  ;[1 1 1] 1. Firstly, lets spawn some subjects, and give them traits to store data in.
  (for _ (range (+ (`self.NumSubjects`) 1))
    (bind _outsubjecthandle (`ApparatusFunctionLibrary.SpawnMachineSubject` 0)) ; Create a new subject
    (`|ExecutionSequence`
      (:`then_0`
        (`|SetSubjectTrait` _outsubjecthandle "/Game/BP_Example/Traits/FBPSubjectPosition.FBPSubjectPosition" (make `/Game/BP_Example/Traits/FBPSubjectPosition` _projectedlocation)) ; Give it a / Set its position
      )
      (:`then_1`
        (`|SetSubjectTrait` _outsubjecthandle "/Game/BP_Example/Traits/FBPDesirespath.FBPDesirespath" (make `/Game/BP_Example/Traits/FBPDesirespath` _projectedlocation)) ; Give it a / Set its position
      ))))

(event `self.ReceiveTick`
  (params (DeltaSeconds :type "Float (single-precision)"))
  (`|ExecutionSequence`
    (:`then_0`
      ;[1 1 1] // Find paths for anyone who currently desires one
      (bind (_subject _subjective _trait_0 _trait_1) (`|Mechanic` "/Game/BP_Example/Traits/FBPDesirespath.FBPDesirespath" "/Game/BP_Example/Traits/FBPSubjectPosition.FBPSubjectPosition")
        (:`Operate`
          (bind _returnvalue (`NavigationSystemV1.FindPathToLocationSynchronously` (`.Value_2_46D0B3754FCB6F913AD782B2A376446F` (break `/Game/BP_Example/Traits/FBPSubjectPosition` _trait_1)) (`.Target_9_46D0B3754FCB6F913AD782B2A376446F` (break `/Game/BP_Example/Traits/FBPDesirespath` _trait_0)) null null)) ; Find a path from the start to the end
          (bind _pathpoints (`NavigationPath.PathPoints` _returnvalue))
          (if (and (`KismetSystemLibrary.IsValid` _returnvalue) (`KismetArrayLibrary.Array_IsValidIndex` _pathpoints))
            (`|ExecutionSequence`
              (:`then_0`
                (`|SetSubjectTrait` _subject "/Game/BP_Example/Traits/FBPHasPath.FBPHasPath" (make `/Game/BP_Example/Traits/FBPHasPath` _pathpoints)) ; Save the path points to a trait
              )
              (:`then_1`
                (`ApparatusFunctionLibrary.RemoveSubjectTrait` _subject "/Game/BP_Example/Traits/FBPDesirespath.FBPDesirespath") ; Remove the desires path trait to prevent frequent planning
              ))
            (else
              (`KismetSystemLibrary.PrintString` "No path found, try again next tick.") ; It might be worth adding a "cooldown" compnent and excluding that from this mechanic to overly frequent path checking
            )))))
    (:`then_1`
      ;[1 1 1] Set desired velocity in the direction of the next path point
      (bind (_subject_2 _subjective_2 _trait_0_2 _trait_1_2) (`|Mechanic` "/Game/BP_Example/Traits/FBPHasPath.FBPHasPath" "/Game/BP_Example/Traits/FBPSubjectPosition.FBPSubjectPosition")
        (:`Operate`
          (bind _output (`|GetArrayItem` (`.Points_11_46D0B3754FCB6F913AD782B2A376446F` (break `/Game/BP_Example/Traits/FBPHasPath` _trait_0_2))))
          (bind _value (break `/Game/BP_Example/Traits/FBPSubjectPosition` _trait_1_2))
          (if (> (`KismetMathLibrary.Vector_Distance` _output _value) (`self.MinGoalDistance`))
            (`|SetSubjectTrait` _subject_2 "/Game/BP_Example/Traits/FBPDesiresVelocity.FBPDesiresVelocity" (make `/Game/BP_Example/Traits/FBPDesiresVelocity` (- _output _value))) ; Set our desired velocity
            (else
              (`KismetSystemLibrary.PrintString` "Close enough to goal point") ; If we're within the minimum distance, we want to remove the 0th position from our path.
              (bind (_out_path _hasanypoints) (`self.WithoutPosZero` _trait_0_2)) ; Takes a path and returns the same path but without pos zero
              (if _hasanypoints
                (`|SetSubjectTrait` _subject_2 "/Game/BP_Example/Traits/FBPHasPath.FBPHasPath" _out_path) ; Update our path with the removed 0th point
                (else
                  (`ApparatusFunctionLibrary.RemoveSubjectTrait` _subject_2 "/Game/BP_Example/Traits/FBPHasPath.FBPHasPath") ; Remove the path entirely
                  (`|SetSubjectTrait` _subject_2 "/Game/BP_Example/Traits/FBPDesiresVelocity.FBPDesiresVelocity" (make `/Game/BP_Example/Traits/FBPDesiresVelocity` (0.0 0.0 0.0))) ; Zero out this subjects velocity trait
                  (`KismetSystemLibrary.PrintString` "This would be a good time to recalculate a path for this subject if they what to loop their movement"))))))))
    (:`then_2`
      ;[1 1 1] Combine desired velocity from pathing with our actual position
      (bind (_subject_3 _subjective_3 _trait_0_3 _trait_1_3) (`|Mechanic` "/Game/BP_Example/Traits/FBPDesiresVelocity.FBPDesiresVelocity" "/Game/BP_Example/Traits/FBPSubjectPosition.FBPSubjectPosition")
        (:`Operate`
          (`|SetSubjectTrait` _subject_3 "/Game/BP_Example/Traits/FBPSubjectPosition.FBPSubjectPosition" (make `/Game/BP_Example/Traits/FBPSubjectPosition` (+ (`.Value_2_46D0B3754FCB6F913AD782B2A376446F` (break `/Game/BP_Example/Traits/FBPSubjectPosition` _trait_1_3)) (* (* (`KismetMathLibrary.Normal` (`.TargetVelocity_10_46D0B3754FCB6F913AD782B2A376446F` (break `/Game/BP_Example/Traits/FBPDesiresVelocity` _trait_0_3))) (`self.SubjectMovespeed`)) (`GameplayStatics.GetWorldDeltaSeconds`))))))))
    (:`then_3`
      ;[1 1 1] 4. This mechanic will debug draw points over all our POSITIONS so we can see whats happpening
      (bind (_subject_4 _subjective_4 _trait_0_4) (`|Mechanic` "/Game/BP_Example/Traits/FBPSubjectPosition.FBPSubjectPosition")
        (:`Operate`
          (`KismetSystemLibrary.DrawDebugPoint` (`.Value_2_46D0B3754FCB6F913AD782B2A376446F` (break `/Game/BP_Example/Traits/FBPSubjectPosition` _trait_0_4)) 20.0 (struct :`G` 1.0 :`A` 1.0)))))
    (:`then_4`
      ;[1 1 1] MECHANIC - Draw some debug information about subjects with paths and positions
      (bind (_subject_5 _subjective_5 _trait_0_5 _trait_1_4) (`|Mechanic` "/Game/BP_Example/Traits/FBPHasPath.FBPHasPath" "/Game/BP_Example/Traits/FBPSubjectPosition.FBPSubjectPosition")
        (:`Operate`
          (bind _points (break `/Game/BP_Example/Traits/FBPHasPath` _trait_0_5))
          (for (_array_element _array_index) _points
            (`KismetSystemLibrary.DrawDebugPoint` _array_element 10.0 (struct :`R` 1.0 :`G` 0.087 :`A` 1.0))
            (`KismetSystemLibrary.DrawDebugLine` (`|GetArrayItem` _points (`KismetMathLibrary.Max` (- _array_index 1))) _array_element (struct :`R` 1.0 :`G` 0.498039 :`A` 1.0) 0.0 5.0))
          (`KismetSystemLibrary.DrawDebugLine` (`.Value_2_46D0B3754FCB6F913AD782B2A376446F` (break `/Game/BP_Example/Traits/FBPSubjectPosition` _trait_1_4)) (`|GetArrayItem` _points) (struct :`R` 1.0 :`G` 0.498039 :`A` 1.0) 0.0 5.0))))))

(fn `UserConstructionScript`)

(fn `WithoutPosZero`
  (params (`In Path` :type "/Game/BP_Example/Traits/FBPHasPath Structure"))
  (returns (`Out Path` :type "/Game/BP_Example/Traits/FBPHasPath Structure") (HasAnyPoints :type Boolean))
  (locals (Local_PathTrait :type "/Game/BP_Example/Traits/FBPHasPath Structure") (Local_PathPoints :type "Array of Vector Structure"))
  (bind _local_pathpoints (`local.Local_PathPoints`))
  (bind _output_get (set `local.Local_PathPoints` (`.Points_11_46D0B3754FCB6F913AD782B2A376446F` (break `/Game/BP_Example/Traits/FBPHasPath` `In Path`))))
  (`KismetArrayLibrary.Array_Remove` _output_get)
  (return (make `/Game/BP_Example/Traits/FBPHasPath` _local_pathpoints) (`KismetArrayLibrary.Array_IsValidIndex` _local_pathpoints)))