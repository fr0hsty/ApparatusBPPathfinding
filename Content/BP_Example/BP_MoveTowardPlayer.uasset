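; Example actor for Apparatus-style subjects, traits and mechanics that makes spawned subjects move toward the player.
; BeginPlay spawns subjects with random, flattened position traits.
; Each Tick, sequenced mechanics save the player's position, step non-player subjects toward it by speed and delta time, then draw debug points at all positions.
; Player and non-players share one position trait, with a Player trait distinguishing them; the lookup assumes a single player.
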(event `self.ReceiveBeginPlay`
  ;[1 1 1] 1. Firstly, lets spawn some subjects, and give them traits to store data in.
  (for _ (range (+ (`self.NumSubjects`) 1))
    (bind _outsubjecthandle (`ApparatusFunctionLibrary.SpawnMachineSubject` 0)) ; Create a new subject
    (`|SetSubjectTrait` _outsubjecthandle "/Game/BP_Example/Traits/FBPSubjectPosition.FBPSubjectPosition" (make `/Game/BP_Example/Traits/FBPSubjectPosition` (* (* (`KismetMathLibrary.RandomUnitVector`) (`self.RandomSpawnWidth`)) (1.0 1.0 0.0)))) ; Give it a / Set its position
  ))

(event `self.ReceiveTick`
  (params (DeltaSeconds :type "Float (single-precision)"))
  (`|ExecutionSequence`
    (:`then_0`
      ;[1 1 1] 2. Grab all subjects with a Player and Position trait.
      ; By default there will only be one of these, so I'm going to save the first one I see ...
      ;
      ; ... But if this was a multiplayer game, there would be more then one - and you would need to create some logic to determine which player you care the most about following.
      ;
      ; NOTE - Inspect the ApparatusThirdPersonCharacter blueprint pawn for more info!
      (bind (_subject _subjective _trait_0 _trait_1) (`|Mechanic` "/Game/BP_Example/Traits/FBPPlayer.FBPPlayer" "/Game/BP_Example/Traits/FBPSubjectPosition.FBPSubjectPosition")
        (:`Operate`
          (bind _output_get (set `self.PlayerPosition` (`.Value_2_46D0B3754FCB6F913AD782B2A376446F` (break `/Game/BP_Example/Traits/FBPSubjectPosition` _trait_1))))
          (`KismetSystemLibrary.PrintString` (`KismetStringLibrary.Concat_StrStr` "Found player position: " (`KismetStringLibrary.Conv_VectorToString` _output_get)) true true (struct :`G` 0.66 :`B` 1.0 :`A` 1.0) 0.0))))
    (:`then_1`
      ;[1 1 1] 3. Move All subjects with a position THAT ARE NOT THE PLAYER toward the player position found above.
      ;
      ; All subjects in this game world use a SubjectPosition trait for their positions. There is no need to have a "player position" and a "NPC position" trait - we can use traits to determine if something is a player or not
      (bind (_subject_2 _subjective_2 _trait_0_2) (`|Mechanic` "/Game/BP_Example/Traits/FBPSubjectPosition.FBPSubjectPosition" "/Game/BP_Example/Traits/FBPPlayer.FBPPlayer")
        (:`Operate`
          (bind _value (break `/Game/BP_Example/Traits/FBPSubjectPosition` _trait_0_2))
          (`|SetSubjectTrait` _subject_2 "/Game/BP_Example/Traits/FBPSubjectPosition.FBPSubjectPosition" (make `/Game/BP_Example/Traits/FBPSubjectPosition` (+ (* (* (`KismetMathLibrary.Normal` (- (`self.PlayerPosition`) _value)) (`GameplayStatics.GetWorldDeltaSeconds`)) (`self.SubjectMovespeed`)) _value))) ; Update the subjects position trait
        )))
    (:`then_2`
      ;[1 1 1] 4. This mechanic will debug draw points over all our POSITIONS so we can see whats happpening
      (bind (_subject_3 _subjective_3 _trait_0_3) (`|Mechanic` "/Game/BP_Example/Traits/FBPSubjectPosition.FBPSubjectPosition")
        (:`Operate`
          (`KismetSystemLibrary.DrawDebugPoint` (`.Value_2_46D0B3754FCB6F913AD782B2A376446F` (break `/Game/BP_Example/Traits/FBPSubjectPosition` _trait_0_3)) 20.0 (struct :`G` 1.0 :`A` 1.0)))))))

(fn `UserConstructionScript`)